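; Manager actor that spawns waves of zombies and tracks their deaths, working with TPSGameModeBase's spawn event and phases.
; SpawnZombie places random pawn classes with a behavior tree inside the StaticMesh bounds, scaling count with TotalWave and binding each OnDeath.
; Tick uses delays to poll death count against spawn count, then switches the game phase.
; DestroyZombies then unpossesses and destroys the AI controllers and resets the counters.
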(event EventBeginPlay
  (bind _astpsgame_mode_base (Utilities|Casting|CastToTPSGameModeBase (Game|GetGameMode)))
  (EventDispatchers|BindEventtoSpawnZombies _astpsgame_mode_base (EventDispatchers|CreateEvent :!event SpawnZombie)))

(event Collision|EventActorBeginOverlap
  (params (OtherActor :type Actor%20Object%20Reference)))

(event EventTick
  (params (DeltaSeconds :type Float%20%28single-precision%29))
  (Utilities|FlowControl|Delay 0.5)
  (if (>= (Variables|Default|GetDeathZombies) (Variables|Default|GetZombieSpawned))
    (bind _astpsgame_mode_base (Utilities|Casting|CastToTPSGameModeBase (Game|GetGameMode)))
    (bind _current_phase (Default|GetCurrentPhase _astpsgame_mode_base))
    (if (Utilities|Enum|Equal(Enum) _current_phase "NewEnumerator1")
      (Utilities|FlowControl|Delay 3.0)
      (Default|SetCurrentPhase _astpsgame_mode_base "NewEnumerator0")
      (CallFunction|DestroyZombies))))

(fn ConstructionScript)

(fn DestroyZombies
  (for _array_element (Variables|Default|GetControllers)
    (bind _astpsaicontroller (Utilities|Casting|CastToTPSAIController (Pawn|GetController _array_element)))
    (Pawn|UnPossess _astpsaicontroller)
    (Actor|DestroyActor _astpsaicontroller)
    (Variables|Default|SetZombieSpawned 0)
    (Variables|Default|SetDeathZombies 0))
  (Utilities|Array|Clear (Variables|Default|GetControllers)))

(fn AddDeathZombie
  (Variables|Default|SetDeathZombies (+ (Variables|Default|GetDeathZombies) 1)))

(fn SpawnZombie
  (bind _staticmesh (Variables|Default|GetStaticMesh))
  (bind (_origin _boxextent) (Collision|GetComponentBounds _staticmesh))
  (bind _astpsgame_mode_base (Utilities|Casting|CastToTPSGameModeBase (Game|GetGameMode)))
  (for _index (range 0 (+ (Variables|/Game/Blueprint/Gameplay/TPSGameModeBase.TPSGameModeBase_C|GetTotal%20Wave _astpsgame_mode_base) 2))
    (Development|PrintString (Utilities|String|ToString(Integer) _index) true true "(R=1.000000,G=0.978449,B=0.000000,A=1.000000)")
    (bind _returnvalue (AI|SpawnAIFromClass (.OutItem (Utilities|Array|Random (Variables|Default|GetRandomPawn))) "/Game/AI/EnemyZombieBT.EnemyZombieBT" (Math|Random|RandomPointinBoundingBox _origin _boxextent) (Math|Rotator|MakeRotator 0.0 0.0 (Math|Random|RandomFloatinRange 0.0 3.6e+02)) false 0))
    (Variables|Default|SetZombieSpawned (+ (Variables|Default|GetZombieSpawned) 1))
    (bind _astpscharacter_base (Utilities|Casting|CastToTPSCharacterBase _returnvalue))
    (EventDispatchers|BindEventtoOnDeath _astpscharacter_base (EventDispatchers|CreateEvent :!event AddDeathZombie))
    (Utilities|Array|Add (Variables|Default|GetControllers) _astpscharacter_base)
    (AI|Components|Blackboard|SetValueasObject (AI|GetBlackboard _returnvalue) (Utilities|Name|MakeLiteralName "SelfActor") _astpscharacter_base))
  (Development|PrintString (Utilities|String|ToString(Integer) (Variables|Default|GetZombieSpawned))))