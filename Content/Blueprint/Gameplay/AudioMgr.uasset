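; Audio manager actor that handles background music for the main menu, shop phase and battle phase.
; On BeginPlay it sets the base sound mix, then fades in menu music on MainMenuLevel or safe-zone music on any other level.
; PlayMusic reads the current phase from TPSGameModeBase and crossfades between safe-zone and battle tracks, fading the outgoing one to near-zero volume.
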(event Custom|Play%20Music
  (bind _astpsgame_mode_base (Utilities|Casting|CastToTPSGameModeBase (Game|GetGameMode)))
  (switch Utilities|FlowControl|Switch|SwitchonGamePhases (Variables|/Game/Blueprint/Gameplay/TPSGameModeBase.TPSGameModeBase_C|GetGame%20Current%20Phase _astpsgame_mode_base)
    (:NewEnumerator0
      (Audio|Components|Audio|FadeOut (Variables|Default|GetBattleMusic) 0.5 0.01 "SCurve" :!class /Script/Engine.AudioComponent)
      (Audio|Components|Audio|FadeIn (Variables|Default|GetSafeZoneMusic) 0.5 0.8 0.0 "Linear" :!class /Script/Engine.AudioComponent))
    (:NewEnumerator1
      (Audio|Components|Audio|FadeIn (Variables|Default|GetBattleMusic) 1.0 0.8 0.0 "SCurve" :!class /Script/Engine.AudioComponent)
      (Audio|Components|Audio|FadeOut (Variables|Default|GetSafeZoneMusic) 1.0 0.01 "SCurve" :!class /Script/Engine.AudioComponent))))

(event EventBeginPlay
  (Class|GameplayStatics|SetBaseSoundMix)
  (bind _returnvalue (Game|GetCurrentLevelName true))
  (if (Utilities|Enum|Equal(Enum) _returnvalue "MainMenuLevel")
    (Audio|Components|Audio|FadeIn (Variables|Default|GetMenuMusic) 0.0 1.0 0.0 "Linear" :!class /Script/Engine.AudioComponent)
    (Audio|Components|Audio|FadeOut (Variables|Default|GetBattleMusic) 0.0 0.0 "Linear" :!class /Script/Engine.AudioComponent)
    (Audio|Components|Audio|FadeOut (Variables|Default|GetSafeZoneMusic) 0.0 0.0 "Linear" :!class /Script/Engine.AudioComponent)
    (else
      (Audio|Components|Audio|FadeIn (Variables|Default|GetSafeZoneMusic) 0.0 1.0 0.0 "Linear" :!class /Script/Engine.AudioComponent)
      (Audio|Components|Audio|FadeOut (Variables|Default|GetBattleMusic) 0.0 0.01 "Linear" :!class /Script/Engine.AudioComponent)
      (Audio|Components|Audio|FadeOut (Variables|Default|GetMenuMusic) 0.0 0.0 "Linear" :!class /Script/Engine.AudioComponent))))

(event Collision|EventActorBeginOverlap
  (params (OtherActor :type Actor%20Object%20Reference)))

(event EventTick
  (params (DeltaSeconds :type Float%20%28single-precision%29)))

(fn ConstructionScript)