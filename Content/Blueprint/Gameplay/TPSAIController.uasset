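; AI controller for TPS characters that runs the possessed character's own behavior tree and, on unpossess, destroys the pawn and stops the tree.
; Sight perception of player pawn 0 sets the blackboard target, or its last known location when lost.
; Hearing writes or clears a sound location key.
; It binds to death events on its pawn and sighted player, with a handler that clears a dead target.
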(event EventPossess
  (params (PossessedPawn :type Pawn%20Object%20Reference))
  (bind _astpscharacter_base (Utilities|Casting|CastToTPSCharacterBase PossessedPawn))
  (Variables|Default|SetPossessed%20TPS%20Character _astpscharacter_base)
  (Utilities|FlowControl|Sequence
    (:then_0
      (CallFunction|RunAI))
    (:then_1
      (bind _possessed_tps_character (Variables|Default|GetPossessed%20TPS%20Character)
        (:then
          (EventDispatchers|BindEventtoOnDeath _possessed_tps_character (EventDispatchers|CreateEvent :!event StopAI)))
        (:else)))))

(event EventUnPossess
  (params (UnpossessedPawn :type Pawn%20Object%20Reference))
  (Utilities|FlowControl|Sequence
    (:then_0
      (bind _possessed_tps_character (Variables|Default|GetPossessed%20TPS%20Character)
        (:then
          (EventDispatchers|UnbindEventfromOnDeath _possessed_tps_character (EventDispatchers|CreateEvent :!event StopAI))
          (Actor|DestroyActor _possessed_tps_character)
          (Variables|Default|SetPossessed%20TPS%20Character 0))
        (:else)))
    (:then_1
      (CallFunction|StopAI))))

(event OnTargetPerceptionUpdated(Sight)
  (params (Actor :type Actor%20Object%20Reference) (Stimulus :type AI%20Stimulus%20Structure))
  (bind _returnvalue (Utilities|Name|MakeLiteralName "Target Last Known Lcoation"))
  (bind _returnvalue_2 (Utilities|Name|MakeLiteralName "Target"))
  (bind _blackboard (Variables|Default|GetBlackboard))
  (bind _blackboard_2 (Variables|Default|GetBlackboard))
  (if (== Actor (Game|Player|GetPlayerPawn 0))
    (if (.bsuccessfullysensed Stimulus)
      (AI|Components|Blackboard|SetValueasObject _blackboard_2 _returnvalue_2 Actor)
      (AI|Components|Blackboard|ClearValue _blackboard _returnvalue)
      (bind _astpscharacter_base (Utilities|Casting|CastToTPSCharacterBase Actor))
      (EventDispatchers|BindEventtoOnDeath _astpscharacter_base (EventDispatchers|CreateEvent :!event HandleTargetDeath))
      (else
        (AI|Components|Blackboard|ClearValue _blackboard_2 _returnvalue_2)
        (AI|Components|Blackboard|SetValueasVector _blackboard _returnvalue (.stimuluslocation Stimulus))))))

(event OnTargetPerceptionUpdated(Hearing)
  (params (Actor :type Actor%20Object%20Reference) (Stimulus :type AI%20Stimulus%20Structure))
  (bind _returnvalue (Utilities|Name|MakeLiteralName "SoundLocation"))
  (bind _blackboard (Variables|Default|GetBlackboard))
  (if (.bsuccessfullysensed Stimulus)
    (AI|Components|Blackboard|SetValueasVector _blackboard _returnvalue (.stimuluslocation Stimulus))
    (else
      (AI|Components|Blackboard|ClearValue _blackboard _returnvalue))))

(fn ConstructionScript)

(fn RunAI
  (bind _possessed_tps_character (Variables|Default|GetPossessed%20TPS%20Character)
    (:then
      (bind _behavior (Variables|/Game/Blueprint/Characters/Abstract/TPSCharacterBase.TPSCharacterBase_C|GetBehavior _possessed_tps_character)
        (:then
          (AI|RunBehaviorTree _behavior))
        (:else)))
    (:else)))

(fn StopAI
  (AI|Logic|StopLogic (Variables|Default|GetBrainComponent) ""))

(fn HandleTargetDeath
  (bind _astpscharacter_base (Utilities|Casting|CastToTPSCharacterBase (AI|Components|Blackboard|GetValueasObject (Variables|Default|GetBlackboard) (Utilities|Name|MakeLiteralName "Target"))))
  (LocalVariables|SetDead%20Character _astpscharacter_base)
  (bind _dead_character (LocalVariables|GetDead%20Character)
    (:then
      (EventDispatchers|UnbindEventfromOnDeath _dead_character (EventDispatchers|CreateEvent :!event HandleTargetDeath))
      (AI|Components|Blackboard|ClearValue (Variables|Default|GetBlackboard) (Utilities|Name|MakeLiteralName "Target")))
    (:else)))