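; Game mode for a third-person shooter with zombie waves, tracking the current game phase.
; After a one-second delay on BeginPlay, it binds an event to the player controller's game mode change.
; ChangePhase moves the game from Shop to Play phase only.
; Entering Play through SetCurrentPhase increments the wave count and calls SpawnZombies.
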(event EventBeginPlay
  (Utilities|FlowControl|Delay 1.0)
  (bind _astpsplayer_controller (Utilities|Casting|CastToTPSPlayerController (Game|GetPlayerController 0)))
  (EventDispatchers|BindEventtoChangeGameMOde _astpsplayer_controller (EventDispatchers|CreateEvent :!event ChangePhase)))

(event EventTick
  (params (DeltaSeconds :type Float%20%28single-precision%29)))

(fn ConstructionScript)

(fn GetCurrentPhase
  (return (Variables|GamePhase|GetGame%20Current%20Phase)))

(fn SetCurrentPhase
  (params (New%20Phase :type GamePhases%20Enum :default "NewEnumerator0"))
  (bind _output_get (Variables|GamePhase|SetGame%20Current%20Phase New%20Phase))
  (switch Utilities|FlowControl|Switch|SwitchonGamePhases _output_get
    (:NewEnumerator1
      (bind _result (Math|Integer|IncrementInt (Variables|GamePhase|GetTotal%20Wave))
        (:%20%20
          (Variables|GamePhase|SetTotal%20Wave _result)
          (Default|CallSpawnZombies))))))

(fn ChangePhase
  (bind _current_phase (CallFunction|GetCurrentPhase))
  (if (Utilities|Enum|Equal(Enum) _current_phase "NewEnumerator0")
    (CallFunction|SetCurrentPhase "NewEnumerator1")))