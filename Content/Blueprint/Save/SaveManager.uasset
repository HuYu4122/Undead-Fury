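; SaveManager loads and saves score entries for the game through a ZombieSave object in a fixed save slot.
; On BeginPlay it loads the existing save, or creates a new one if loading or casting fails, and sets the write index to the end of the Scores array.
; Save writes an entry at that fixed index, so repeated calls overwrite it, then writes the slot and prints success or failure.
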(event EventBeginPlay
  (bind _returnvalue (SaveGame|LoadGamefromSlot "slot0"))
  (Utilities|IsValid _returnvalue
    (:Is%20Valid
      (bind _aszombie_save (Utilities|Casting|CastToZombieSave _returnvalue)
        (:then
          (bind _output_get (Variables|Default|SetCurrent%20Save%20Game _aszombie_save))
          (Variables|Default|SetIndex (Utilities|Array|Length (Variables|/Game/Blueprint/Save/ZombieSave.ZombieSave_C|GetScores _output_get))))
        (:CastFailed
          (bind _returnvalue_2 (SaveGame|CreateSaveGameObject "/Game/Blueprint/Save/ZombieSave.ZombieSave_C" :!label _label))
          (Variables|Default|SetCurrent%20Save%20Game _returnvalue_2)
          (Variables|Default|SetIndex 0))))
    (:Is%20Not%20Valid
      (goto _label))))

(fn ConstructionScript)

(fn Save
  (params (Save :type Save%20Struct%20Structure))
  (bind _current_save_game (Variables|Default|GetCurrent%20Save%20Game))
  (Utilities|Array|SetArrayElem (Variables|/Game/Blueprint/Save/ZombieSave.ZombieSave_C|GetScores _current_save_game) (Variables|Default|GetIndex) Save true)
  (bind _returnvalue (SaveGame|SaveGametoSlot _current_save_game "slot0"))
  (if _returnvalue
    (Development|PrintText "SAVED!" true true "(R=0.000000,G=1.000000,B=0.039678,A=1.000000)")
    (else
      (Development|PrintText "SAVE FAILED!" true true "(R=1.000000,G=0.000000,B=0.025978,A=1.000000)"))))