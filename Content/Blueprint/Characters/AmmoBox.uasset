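; Ammo box actor that refills the player's equipped weapon as soon as it begins play, with no overlap trigger.
; BeginPlay casts player 0 to TPSCharacterBase and passes its equipped weapon to RechargeWeapon.
; RechargeWeapon ignores that input, fetches the weapon again and sets ActualBullets to MunitionsInMagazine unless the count is already higher.
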(event EventBeginPlay
  (bind _astpscharacter_base (Utilities|Casting|CastToTPSCharacterBase (Game|GetPlayerCharacter 0)))
  (CallFunction|RechargeWeapon (Default|GetEquippedWeapon _astpscharacter_base)))

(event Collision|EventActorBeginOverlap
  (params (OtherActor :type Actor%20Object%20Reference)))

(event EventTick
  (params (DeltaSeconds :type Float%20%28single-precision%29)))

(fn ConstructionScript)

(fn RechargeWeapon
  (params (EquippedWeapon :type Weapon%20Object%20Reference))
  (bind _munitionsinmagazine (Variables|Default|GetMunitionsInMagazine))
  (bind _astpscharacter_base (Utilities|Casting|CastToTPSCharacterBase (Game|GetPlayerCharacter 0)))
  (if (not (> (Variables|/Game/Blueprint/Weapons/Abstract/Weapon.Weapon_C|GetActualBullets (Default|GetEquippedWeapon _astpscharacter_base)) _munitionsinmagazine))
    (Variables|/Game/Blueprint/Weapons/Abstract/Weapon.Weapon_C|SetActualBullets (Default|GetEquippedWeapon _astpscharacter_base) _munitionsinmagazine)))