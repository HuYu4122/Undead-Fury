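; AmmoBox is an item that adds ammo to the player's equipped weapon as soon as it begins play, with no overlap trigger.
; BeginPlay casts player character 0 to TPSCharacterBase and calls RechargeWeapon, which adds Ammo to the weapon's ActualBullets, capped at MaxBullets.
; RechargeWeapon ignores its EquippedWeapon input and fetches the weapon from the player again.
; The box never destroys itself in these graphs.
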(event EventBeginPlay
  (bind _astpscharacter_base (Utilities|Casting|CastToTPSCharacterBase (Game|GetPlayerCharacter 0)))
  (CallFunction|RechargeWeapon (Default|GetEquippedWeapon _astpscharacter_base)))

(event Collision|EventActorBeginOverlap
  (params (OtherActor :type Actor%20Object%20Reference)))

(event EventTick
  (params (DeltaSeconds :type Float%20%28single-precision%29)))

(fn ConstructionScript)

(fn RechargeWeapon
  (params (EquippedWeapon :type Weapon%20Object%20Reference))
  (bind _astpscharacter_base (Utilities|Casting|CastToTPSCharacterBase (Game|GetPlayerCharacter 0)))
  (if (>= (+ (Variables|/Game/Blueprint/Weapons/Abstract/Weapon.Weapon_C|GetActual%20Bullets (Default|GetEquippedWeapon _astpscharacter_base)) (Variables|Default|GetAmmo)) (Variables|/Game/Blueprint/Weapons/Abstract/Weapon.Weapon_C|GetMax%20Bullets (Default|GetEquippedWeapon _astpscharacter_base)))
    (Variables|/Game/Blueprint/Weapons/Abstract/Weapon.Weapon_C|SetActual%20Bullets (Default|GetEquippedWeapon _astpscharacter_base) (Variables|/Game/Blueprint/Weapons/Abstract/Weapon.Weapon_C|GetMax%20Bullets (Default|GetEquippedWeapon _astpscharacter_base)))
    (else
      (Variables|/Game/Blueprint/Weapons/Abstract/Weapon.Weapon_C|SetActual%20Bullets (Default|GetEquippedWeapon _astpscharacter_base) (+ (Variables|/Game/Blueprint/Weapons/Abstract/Weapon.Weapon_C|GetActual%20Bullets (Default|GetEquippedWeapon _astpscharacter_base)) (Variables|Default|GetAmmo))))))