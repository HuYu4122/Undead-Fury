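; Actor component that tracks an owner's health, with damage, cure and alive or current-health queries.
; Health starts at a fixed value on BeginPlay, and Damage lowers it with a floor at zero.
; Damage broadcasts OnChanged only when the value actually changes, then OnDeath if it reaches zero.
; Cure restores MaxHealth directly without broadcasting a change.
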(event Custom|Cure
  (Variables|Health|SetCurrent%20Health (Variables|Health|GetMax%20Health)))

(event EventBeginPlay
  (Variables|Health|SetCurrent%20Health 5e+01))

(fn Damage
  (params (Damage%20Amount :type Float%20%28double-precision%29))
  (LocalVariables|SetPrev%20Health (Variables|Health|GetCurrent%20Health))
  (bind _output_get (Variables|Health|SetCurrent%20Health (Math|Float|Max(Float) (- (Variables|Health|GetCurrent%20Health) Damage%20Amount) 0.0)))
  (if (!= _output_get (LocalVariables|GetPrev%20Health))
    ;[1 1 1] All this happens only if health changed
    (Default|CallOnChanged self (LocalVariables|GetPrev%20Health) (Variables|Health|GetCurrent%20Health))
    (if (<= (Variables|Health|GetCurrent%20Health) 0.0)
      (Default|CallOnDeath self))))

(fn IsAlive
  (return (> (Variables|Health|GetCurrent%20Health) 0.0)))

(fn GetCurrentHealth
  (return (Variables|Health|GetCurrent%20Health)))